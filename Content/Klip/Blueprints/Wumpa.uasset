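; Wumpa fruit collectible that raises the player's Wumpa count when picked up.
; Until collected, it rotates every tick and bobs using offsets from the KeySpin timeline.
; Any overlap with its sphere destroys it, increments player 0's counter, plays a 2D sound and refreshes the HUD total through the game mode.
; The overlap handler does not check which actor entered.
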(event OnComponentBeginOverlap(Sphere)
  (params (OverlappedComponent :type Primitive%20Component%20Object%20Reference) (OtherActor :type Actor%20Object%20Reference) (OtherComp :type Primitive%20Component%20Object%20Reference) (OtherBodyIndex :type Integer) (bFromSweep :type Boolean) (SweepResult :type Hit%20Result%20Structure%20%28by%20ref%29))
  (Actor|DestroyActor)
  (bind _ascoffee_bandicoot_player (Utilities|Casting|CastToCoffeeBandicootPlayer (Game|GetPlayerCharacter 0)))
  (Math|Integer|IncrementInt (Variables|/Game/CoffeeBandicoot/Blueprints/CoffeeBandicootPlayer.CoffeeBandicootPlayer_C|GetNumberOfWumpa _ascoffee_bandicoot_player)
    (:%20%20
      (Audio|PlaySound2D "/Game/CoffeeBandicoot/Audio/Wumpa.Wumpa" 1.0 1.0 0.0 0 0)
      (Variables|Default|SetWumpaDestroyed true)
      (bind _ascoffee_bandicoot_game_mode (Utilities|Casting|CastToCoffeeBandicootGameMode (Game|GetGameMode)))
      (Default|UpdateWumpaTotal (Variables|/Game/Klip/Blueprints/CoffeeBandicootGameMode.CoffeeBandicootGameMode_C|GetHUD _ascoffee_bandicoot_game_mode)))))

(event EventTick
  (params (DeltaSeconds :type Float%20%28single-precision%29))
  (if (not (Variables|Default|GetWumpaDestroyed))
    (Transformation|AddActorLocalRotation "0,2.500000, 0" false false)
    (bind _wumpafruitbounce (Timeline|KeySpin Play)
      (:Update
        (Transformation|AddActorLocalOffset _wumpafruitbounce false false)))))

(fn ConstructionScript)